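; In-game player controller that requests the player's pawn spawn and manages their match UI.
; On BeginPlay it loads the saved player info, passes it to GameGM_BP through SendInfoToServer for spawning, then re-saves it.
; Events create the game HUD, loading screen and team victory widgets, and feed kill messages into the HUD.
; Tick shrinks other pawns' health/nickname widgets with distance from the controlled pawn and prunes invalid pawns.
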(event `SendInfoToServer`
  (params (Playerinfo :type "/Game/TopoGra/Blueprints/PlayerInfo_Struct Structure"))
  (`/Game/TopoGra/Blueprints/Game/GameGM_BP.RequestSpawningPawn` (cast `/Game/TopoGra/Blueprints/Game/GameGM_BP` (`GameplayStatics.GetGameMode`) :!pure true) self Playerinfo))

(event `FirstLoadGame`
  (bind _returnvalue (`GameplayStatics.LoadGameFromSlot` (`self.MySaveSlotName`)))
  (`/Engine/EditorBlueprintResources/StandardMacros.IsValid` _returnvalue
    (:`Is Valid`
      (bind _asplayer_info_save_bp (cast `/Game/TopoGra/Save/PlayerInfoSave_BP` _returnvalue))
      (`self.SendInfoToServer` (`/Game/TopoGra/Save/PlayerInfoSave_BP.PlayerInfo` _asplayer_info_save_bp))
      (`GameplayStatics.SaveGameToSlot` _asplayer_info_save_bp (`self.MySaveSlotName`)))
    (:`Is Not Valid`
      (`KismetSystemLibrary.PrintString` "error Loading game" true true (struct :`R` 1.0 :`A` 1.0) 100.0))))

(event `self.ReceiveBeginPlay`
  (`self.FirstLoadGame`))

(event `RemoveWidgets`
  (`WidgetLayoutLibrary.RemoveAllWidgets`))

(event `CreateGameWidget`
  (params (TimeLeft :type "Float (double-precision)"))
  (`WidgetLayoutLibrary.RemoveAllWidgets`)
  (bind _returnvalue (`|CreateWidget` "/Game/TopoGra/Widgets/Game_WBP.Game_WBP_C" self TimeLeft))
  (set `self.GameWidget` _returnvalue)
  (`UserWidget.AddToViewport` _returnvalue 0))

(event `self.ReceiveTick`
  (params (DeltaSeconds :type "Float (single-precision)"))
  (bind _playerspawns (`self.PlayersPawns`))
  (for _array_element _playerspawns
    (`/Engine/EditorBlueprintResources/StandardMacros.IsValid` _array_element
      (:`Is Valid`
        (bind _returnvalue (`WidgetComponent.GetUserWidgetObject` (`/Game/TopoGra/Blueprints/Player/PlayerCharacter_BP.HealthNickWidget` _array_element)))
        (`/Engine/EditorBlueprintResources/StandardMacros.IsValid` _returnvalue
          (:`Is Valid`
            (bind _returnvalue_2 (`KismetMathLibrary.MapRangeClamped` (`self.GetDistanceTo` _array_element (`self.K2_GetPawn`)) 100.0 6000.0 1.0 0.2))
            (`Widget.SetRenderScale` (cast `/Game/TopoGra/Widgets/InGamePlayer_WBP` _returnvalue :!pure true) (`KismetMathLibrary.MakeVector2D` _returnvalue_2 _returnvalue_2)))))
      (:`Is Not Valid`
        (`KismetArrayLibrary.Array_RemoveItem` _playerspawns _array_element)))))

(event `AddLoadingScreen`
  (bind _returnvalue (`|CreateWidget` "/Game/TopoGra/Widgets/LoadingScreen.LoadingScreen_C" self))
  (`UserWidget.AddToViewport` _returnvalue 0))

(event `AddKillTextPC`
  (params (KillText :type Text))
  (`/Game/TopoGra/Widgets/Game_WBP.AddToKills` (`self.GameWidget`) KillText))

(event `AddBlueVictoryWidget`
  (bind _returnvalue (`|CreateWidget` "/Game/TopoGra/Widgets/Victory_WBP.Victory_WBP_C" (`GameplayStatics.GetPlayerController` 0) "BLUE"))
  (`UserWidget.AddToViewport` _returnvalue 0))

(event `AddRedVictoryWidget`
  (bind _returnvalue (`|CreateWidget` "/Game/TopoGra/Widgets/Victory_WBP.Victory_WBP_C" (`GameplayStatics.GetPlayerController` 0) "RED"))
  (`UserWidget.AddToViewport` _returnvalue 0))

(fn `UserConstructionScript`)