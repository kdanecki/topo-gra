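; Spectator pawn that lets a player watch living teammates on its Red or Blue Side through their cameras.
; On possession it creates the observer widget for the controlling player.
; Observe snaps it to the target's camera and moves it between players' Observers lists.
; PreviousPlayer and NextPlayer step through the GameMode's alive-side array, though their wrap-around checks are faulty at the list ends.
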(event `Observe`
  (params (Player :type "/Game/TopoGra/Blueprints/Player/PlayerCharacter_BP Object Reference"))
  (bind _currentlyobserving (`self.CurrentlyObserving`))
  (`/Engine/EditorBlueprintResources/StandardMacros.IsValid` _currentlyobserving
    (:`Is Valid`
      (`KismetArrayLibrary.Array_RemoveItem` (`/Game/TopoGra/Blueprints/Player/PlayerCharacter_BP.Observers` _currentlyobserving) self))
    (:`Is Not Valid`
      _))
  (`self.K2_AttachToComponent` (`/Game/TopoGra/Blueprints/Player/PlayerCharacter_BP.Camera` Player) "None" "SnapToTarget" "SnapToTarget" "KeepRelative")
  (set `self.CurrentlyObserving` Player)
  (`KismetArrayLibrary.Array_Add` (`/Game/TopoGra/Blueprints/Player/PlayerCharacter_BP.Observers` Player) self))

(event `self.ReceivePossessed`
  (params (NewController :type "Controller Object Reference"))
  (bind _asplayer_controller (cast `PlayerController` NewController))
  (bind _returnvalue (`|CreateWidget` "/Game/TopoGra/Widgets/ObserverWidget.ObserverWidget_C" _asplayer_controller))
  (`UserWidget.AddToViewport` _returnvalue 0))

(event `PreviousPlayer`
  (bind _asgame_gm_bp (cast `/Game/TopoGra/Blueprints/Game/GameGM_BP` (`GameplayStatics.GetGameMode`) :!pure true))
  (bind _aliveredside (`/Game/TopoGra/Blueprints/Game/GameGM_BP.AliveRedSide` _asgame_gm_bp))
  (bind _aliveblueside (`/Game/TopoGra/Blueprints/Game/GameGM_BP.AliveBlueSide` _asgame_gm_bp))
  (bind _returnvalue (- (`KismetArrayLibrary.Array_Find` _aliveredside (`self.CurrentlyObserving`)) 1))
  (bind _returnvalue_2 (- (`KismetArrayLibrary.Array_Find` _aliveblueside (`self.CurrentlyObserving`)) 1))
  (switch `string` (`self.Side`)
    (:`Red`
      (if (< _returnvalue 0)
        (`self.Observe` (`|GetArrayItem` _aliveredside _returnvalue))
        (else
          (`self.Observe` (`|GetArrayItem` _aliveredside (- (`KismetArrayLibrary.Array_Length` _aliveredside) 1))))))
    (:`Blue`
      (if (< _returnvalue_2 0)
        (`self.Observe` (`|GetArrayItem` _aliveblueside _returnvalue_2))
        (else
          (`self.Observe` (`|GetArrayItem` _aliveblueside (- (`KismetArrayLibrary.Array_Length` _aliveblueside) 1))))))))

(event `NextPlayer`
  (bind _asgame_gm_bp (cast `/Game/TopoGra/Blueprints/Game/GameGM_BP` (`GameplayStatics.GetGameMode`) :!pure true))
  (bind _aliveredside (`/Game/TopoGra/Blueprints/Game/GameGM_BP.AliveRedSide` _asgame_gm_bp))
  (bind _aliveblueside (`/Game/TopoGra/Blueprints/Game/GameGM_BP.AliveBlueSide` _asgame_gm_bp))
  (bind _returnvalue (+ (`KismetArrayLibrary.Array_Find` _aliveredside (`self.CurrentlyObserving`)) 1))
  (bind _returnvalue_2 (+ (`KismetArrayLibrary.Array_Find` _aliveblueside (`self.CurrentlyObserving`)) 1))
  (switch `string` (`self.Side`)
    (:`Red`
      (if (> _returnvalue (`KismetArrayLibrary.Array_Length` _aliveredside))
        (`self.Observe` (`|GetArrayItem` _aliveredside))
        (else
          (`self.Observe` (`|GetArrayItem` _aliveredside _returnvalue)))))
    (:`Blue`
      (if (> _returnvalue_2 (`KismetArrayLibrary.Array_Length` _aliveblueside))
        (`self.Observe` (`|GetArrayItem` _aliveblueside))
        (else
          (`self.Observe` (`|GetArrayItem` _aliveblueside _returnvalue_2)))))))

(fn `UserConstructionScript`)