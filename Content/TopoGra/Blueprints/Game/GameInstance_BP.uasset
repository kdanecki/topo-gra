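; Game instance Blueprint that handles menu screens and online session hosting and joining.
; Show events display the main menu, play and lobby widgets, caching each on first creation and enabling the mouse cursor.
; HostGame creates a non-LAN session, then opens the lobby level as a listen server.
; JoinGame searches for a single session and joins that result, printing whether the join succeeded.
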(event `ShowMainMenu`
  (bind _returnvalue (`GameplayStatics.GetPlayerController` 0))
  (bind _mainmenu_ref (`self.MainMenu_Ref`))
  (`/Engine/EditorBlueprintResources/StandardMacros.IsValid` _mainmenu_ref
    (:`Is Valid`
      (`UserWidget.AddToViewport` _mainmenu_ref 0))
    (:`Is Not Valid`
      (bind _returnvalue_2 (`|CreateWidget` "/Game/TopoGra/Widgets/MainMenu_WBP.MainMenu_WBP_C" _returnvalue))
      (bind _output_get (set `self.MainMenu_Ref` _returnvalue_2))
      (`UserWidget.AddToViewport` _output_get 0)))
  (set `PlayerController.bShowMouseCursor` true _returnvalue))

(event `HostGame`
  ;[1 1 1] Host / Join
  (`KismetSystemLibrary.PrintString` "Host")
  (`CreateSessionCallbackProxy.CreateSession` (`GameplayStatics.GetPlayerController` 0) 11
    (:`OnSuccess`
      (`GameplayStatics.OpenLevel` "Lobby_L" true "listen"))))

(event `ShowPlayWidget`
  (bind _returnvalue (`GameplayStatics.GetPlayerController` 0))
  (`/Engine/EditorBlueprintResources/StandardMacros.IsValid` (`self.JoiningWidget_Ref`)
    (:`Is Valid`
      (`UserWidget.AddToViewport` (`self.JoiningWidget_Ref`) 0)
      (set `PlayerController.bShowMouseCursor` true _returnvalue))
    (:`Is Not Valid`
      (bind _returnvalue_2 (`|CreateWidget` "/Game/TopoGra/Widgets/Play_WBP.Play_WBP_C" _returnvalue))
      (bind _output_get (set `self.JoiningWidget_Ref` _returnvalue_2))
      (`UserWidget.AddToViewport` _output_get 0)
      (set `PlayerController.bShowMouseCursor` true _returnvalue))))

(event `JoinGame`
  (bind _returnvalue (`GameplayStatics.GetPlayerController` 0))
  ;[1 1 1] Host / Join
  (bind _results (`FindSessionsCallbackProxy.FindSessions` _returnvalue 1)
    (:`OnSuccess`
      (`JoinSessionCallbackProxy.JoinSession` _returnvalue (`|GetArrayItem` _results)
        (:`OnSuccess`
          (`KismetSystemLibrary.PrintString` "joined"))
        (:`OnFailure`
          (`KismetSystemLibrary.PrintString` "failed to join"))))))

(event `ShowLobbyWidget`
  (bind _returnvalue (`GameplayStatics.GetPlayerController` 0))
  (`/Engine/EditorBlueprintResources/StandardMacros.IsValid` (`self.LobbyWidget_Ref`)
    (:`Is Valid`
      (`UserWidget.AddToViewport` (`self.LobbyWidget_Ref`) 0)
      (set `PlayerController.bShowMouseCursor` true _returnvalue))
    (:`Is Not Valid`
      (bind _returnvalue_2 (`|CreateWidget` "/Game/TopoGra/Widgets/Lobby_WBP.Lobby_WBP_C" _returnvalue))
      (bind _output_get (set `self.LobbyWidget_Ref` _returnvalue_2))
      (`UserWidget.AddToViewport` _output_get 0)
      (set `PlayerController.bShowMouseCursor` true _returnvalue))))