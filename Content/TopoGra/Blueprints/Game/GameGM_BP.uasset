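; Game mode for a two-team Red versus Blue elimination match with admin observers.
; A start timer, whose match-start event is empty, feeds the countdown to each player's game widget after login.
; Loaded players move to free side-tagged PlayerStarts and join alive lists, while Observers possess a spawned admin pawn.
; Deaths update kill feeds, retarget spectators and print wins, though Blue deaths mistakenly remove from the Red list.
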(event `self.K2_OnSwapPlayerControllers`
  (params (OldPC :type "PlayerController Object Reference") (NewPC :type "PlayerController Object Reference"))
  (`KismetSystemLibrary.PrintString` "SWAPPED" true true (struct :`G` 0.014998 :`B` 1.0 :`A` 1.0)))

(event `self.ReceiveBeginPlay`
  (`KismetSystemLibrary.PrintString` "this is gamemode")
  (bind _returnvalue (`KismetSystemLibrary.K2_SetTimerDelegate` (delegate `StartTheMatch`) (`self.StartDelay`)))
  (set `self.StartTimer` _returnvalue)
  (bind _outactors (`GameplayStatics.GetAllActorsOfClass` "/Script/Engine.PlayerStart"))
  (set `self.FreePlayerStarts` _outactors))

(event `StartTheMatch`)

(event `self.K2_PostLogin`
  (params (NewPlayer :type "PlayerController Object Reference"))
  (bind _starttimer (`self.StartTimer`))
  (bind _starttimer_2 (`self.StartTimer`))
  (bind _asgame_player_controller_bp (cast `/Game/TopoGra/Blueprints/Player/GamePlayerController_BP` NewPlayer)
    (:`then`
      (`KismetArrayLibrary.Array_Add` (`self.PlayersControllers`) _asgame_player_controller_bp)
      (if (`KismetSystemLibrary.K2_IsTimerActiveHandle` _starttimer_2)
        (`/Game/TopoGra/Blueprints/Player/GamePlayerController_BP.CreateGameWidget` _asgame_player_controller_bp (`KismetSystemLibrary.K2_GetTimerRemainingTimeHandle` _starttimer_2))
        (else
          (`KismetSystemLibrary.Delay` 1.0)
          (if (`KismetSystemLibrary.K2_IsTimerActiveHandle` _starttimer)
            (`/Game/TopoGra/Blueprints/Player/GamePlayerController_BP.CreateGameWidget` _asgame_player_controller_bp (`KismetSystemLibrary.K2_GetTimerRemainingTimeHandle` _starttimer))
            (else
              (`/Game/TopoGra/Blueprints/Player/GamePlayerController_BP.CreateGameWidget` _asgame_player_controller_bp 0.0))))))
    (:`CastFailed`
      (`KismetSystemLibrary.PrintString` "wrong controller"))))

(event `PlayerSentLoadedInfo`
  (params (Player :type "/Game/TopoGra/Blueprints/Player/PlayerCharacter_BP Object Reference") (Controller :type "/Game/TopoGra/Blueprints/Player/GamePlayerController_BP Object Reference") (Side :type String))
  (bind _freeplayerstarts (`self.FreePlayerStarts`))
  (bind _freeplayerstarts_2 (`self.FreePlayerStarts`))
  (if (`KismetStringLibrary.EqualEqual_StrStr` Side "Red")
    (for _array_element _freeplayerstarts
      (if (== (`PlayerStart.PlayerStartTag` _array_element) "Red")
        (`self.K2_SetActorTransform` Player (`self.GetTransform` _array_element) false false)
        (`KismetArrayLibrary.Array_RemoveItem` _freeplayerstarts _array_element)
        (`KismetArrayLibrary.Array_Add` (`self.AliveRedSide`) Player)
        (`KismetSystemLibrary.PrintString` "red")
        (break)))
    (elif (`KismetStringLibrary.EqualEqual_StrStr` Side "Blue")
      (for _array_element_2 _freeplayerstarts_2
        (if (== (`PlayerStart.PlayerStartTag` _array_element_2) "Blue")
          (`self.K2_SetActorTransform` Player (`self.GetTransform` _array_element_2) false false)
          (`KismetArrayLibrary.Array_RemoveItem` _freeplayerstarts_2 _array_element_2)
          (`KismetArrayLibrary.Array_Add` (`self.AliveBlueSide`) Player)
          (`KismetSystemLibrary.PrintString` "blue")
          (break)))
      (elif (`KismetStringLibrary.EqualEqual_StrStr` Side "Observer")
        (`self.K2_DestroyActor` Player)
        (`/Game/TopoGra/Blueprints/Player/GamePlayerController_BP.RemoveWidgets` Controller)
        (for _array_element_3 (`self.FreePlayerStarts`)
          (if (== (`PlayerStart.PlayerStartTag` _array_element_3) "Admin")
            (bind _returnvalue (`|SpawnActorFromClass` "/Game/TopoGra/Blueprints/Player/AdminObserver_BP.AdminObserver_BP_C" (`self.GetTransform` _array_element_3) "Undefined" "OverrideRootScale" null null))
            (`Controller.Possess` Controller _returnvalue)
            (`KismetSystemLibrary.PrintString` "observe")
            (break)))))))

(event `CharacterDied`
  (params (Character :type "/Game/TopoGra/Blueprints/Player/PlayerCharacter_BP Object Reference") (NewObserver :type "/Game/TopoGra/Blueprints/Player/PlayerObserver_BP Object Reference") (KillText :type Text))
  (bind _side (`/Game/TopoGra/Blueprints/Player/PlayerCharacter_BP.Side` Character))
  (bind _aliveredside (`self.AliveRedSide`))
  (bind _output (`|GetArrayItem` (`self.AliveBlueSide`)))
  (bind _output_2 (`|GetArrayItem` (`self.AliveRedSide`)))
  (for _array_element (`self.PlayersControllers`)
    (bind _gamewidget (`/Game/TopoGra/Blueprints/Player/GamePlayerController_BP.GameWidget` _array_element))
    (`/Engine/EditorBlueprintResources/StandardMacros.IsValid` _gamewidget
      (:`Is Valid`
        (`/Game/TopoGra/Widgets/Game_WBP.AddToKills` _gamewidget KillText))))
  (if (`KismetStringLibrary.EqualEqual_StrStr` _side "Red")
    (`KismetArrayLibrary.Array_RemoveItem` _aliveredside Character)
    (if (<= (`KismetArrayLibrary.Array_Length` (`self.AliveRedSide`)) 0)
      (`self.BlueWon`)
      (else
        (`/Game/TopoGra/Blueprints/Player/PlayerObserver_BP.Observe` NewObserver _output_2)
        (for _array_element_2 (`/Game/TopoGra/Blueprints/Player/PlayerCharacter_BP.Observers` Character)
          (`/Game/TopoGra/Blueprints/Player/PlayerObserver_BP.Observe` _array_element_2 _output_2))))
    (elif (`KismetStringLibrary.EqualEqual_StrStr` _side "Blue")
      (`KismetArrayLibrary.Array_RemoveItem` _aliveredside Character)
      (if (<= (`KismetArrayLibrary.Array_Length` (`self.AliveBlueSide`)) 0)
        (`self.RedWon`)
        (else
          (`/Game/TopoGra/Blueprints/Player/PlayerObserver_BP.Observe` NewObserver _output)
          (for _array_element_3 (`/Game/TopoGra/Blueprints/Player/PlayerCharacter_BP.Observers` Character)
            (`/Game/TopoGra/Blueprints/Player/PlayerObserver_BP.Observe` _array_element_3 _output)))))))

(event `BlueWon`
  (`KismetSystemLibrary.PrintString` "blue won"))

(event `RedWon`
  (`KismetSystemLibrary.PrintString` "red won"))

(fn `UserConstructionScript`)