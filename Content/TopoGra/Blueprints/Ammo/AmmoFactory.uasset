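; AmmoFactory is an actor that produces ammo at its own location on a repeating timer.
; On BeginPlay it starts a looping timer at the Speed interval and runs Produce once immediately.
; Produce adds AmountAtOnce to the tracked ammo pickup while it is valid, otherwise it spawns a new Ammo_BP of the configured AmmoType and tracks that.
; A leftover debug "Hello" prints on every production.
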(event `self.ReceiveBeginPlay`
  (`self.StartProduction`))

(event `StartProduction`
  (bind _returnvalue (`KismetSystemLibrary.K2_SetTimerDelegate` (delegate `Produce`) (`self.Speed`) true))
  (set `self.Timer` _returnvalue)
  (`self.Produce`))

(event `Produce`
  (bind _currentammo_ref (`self.CurrentAmmo_Ref`))
  (`KismetSystemLibrary.PrintString` "Hello")
  (`/Engine/EditorBlueprintResources/StandardMacros.IsValid` (`self.CurrentAmmo_Ref`)
    (:`Is Valid`
      (set `/Game/TopoGra/Blueprints/Ammo/Ammo_BP.Amount` (+ (`/Game/TopoGra/Blueprints/Ammo/Ammo_BP.Amount` _currentammo_ref) (`self.AmountAtOnce`)) _currentammo_ref))
    (:`Is Not Valid`
      (bind _returnvalue (`|SpawnActorFromClass` "/Game/TopoGra/Blueprints/Ammo/Ammo_BP.Ammo_BP_C" (`KismetMathLibrary.MakeTransform` (+ (`self.K2_GetActorLocation`) (0.0 0.0 0.0)) (`self.K2_GetActorRotation`)) "Undefined" "OverrideRootScale" null (`self.AmmoType`) null))
      (set `/Game/TopoGra/Blueprints/Ammo/Ammo_BP.Amount` (`self.AmountAtOnce`) _returnvalue)
      (set `self.CurrentAmmo_Ref` _returnvalue))))

(fn `UserConstructionScript`)