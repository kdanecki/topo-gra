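; LobbyPC_BP is the lobby player controller that handles a player's saved info, lobby UI and requests to the game mode.
; InitialSetup loads PlayerInfo from a PlayerInfoSave_BP slot, passes it to SendInfoToServer to store as MyPlayerInfo, then creates the Lobby_WBP widget.
; UpdateWidget forwards all players' info to that widget, and a separate event shows a loading screen.
; Server-named events call LobbyGM to refresh everyone or start the game.
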(event `SendInfoToServer`
  (params (NewParam :type "/Game/TopoGra/Blueprints/PlayerInfo_Struct Structure"))
  (set `self.MyPlayerInfo` NewParam))

(event `AddWidget`
  (bind _returnvalue (`|CreateWidget` "/Game/TopoGra/Widgets/Lobby_WBP.Lobby_WBP_C" self))
  (set `self.LobbyWidget_Ref` _returnvalue)
  (`UserWidget.AddToViewport` _returnvalue 0))

(event `InitialSetup`
  (`self.RefreshSave`)
  (`self.AddWidget`))

(event `AddLoadingScreen`
  (bind _returnvalue (`|CreateWidget` "/Game/TopoGra/Widgets/LoadingScreen.LoadingScreen_C" self))
  (`UserWidget.AddToViewport` _returnvalue 0))

(event `RefreshSave`
  (bind _loadedinfo (`self.LoadGame`))
  (`self.SendInfoToServer` _loadedinfo))

(event `UpdateWidget`
  (params (AllPlayersInfo :type "Array of /Game/TopoGra/Blueprints/PlayerInfo_Struct Structure"))
  (`/Game/TopoGra/Widgets/Lobby_WBP.UpdateWidget` (`self.LobbyWidget_Ref`) AllPlayersInfo))

(event `TellServerToUpdateEveryone`
  (`/Game/TopoGra/Blueprints/Lobby/LobbyGM.EveryoneUpdate` (cast `/Game/TopoGra/Blueprints/Lobby/LobbyGM` (`GameplayStatics.GetGameMode`) :!pure true)))

(event `TellServerToStart`
  (`self.StartGame`))

(event `StartGame`
  (`/Game/TopoGra/Blueprints/Lobby/LobbyGM.StartTheGame` (cast `/Game/TopoGra/Blueprints/Lobby/LobbyGM` (`GameplayStatics.GetGameMode`) :!pure true)))

(fn `LoadGame`
  (returns (LoadedInfo :type "/Game/TopoGra/Blueprints/PlayerInfo_Struct Structure"))
  (bind _returnvalue (`GameplayStatics.LoadGameFromSlot` (`self.MySaveSlotName`)))
  (`/Engine/EditorBlueprintResources/StandardMacros.IsValid` _returnvalue
    (:`Is Valid`
      (bind _asplayer_info_save_bp (cast `/Game/TopoGra/Save/PlayerInfoSave_BP` _returnvalue))
      (bind _playerinfo (`/Game/TopoGra/Save/PlayerInfoSave_BP.PlayerInfo` _asplayer_info_save_bp))
      (set `self.LoadedInfo` _playerinfo)
      (`KismetSystemLibrary.PrintString` (`KismetStringLibrary.Concat_StrStr` (`KismetTextLibrary.Conv_TextToString` (`.Nickname_2_D23EF68447AA44EF44A67B84BE2175FE` (break `/Game/TopoGra/Blueprints/PlayerInfo_Struct` _playerinfo))) " added nickname") true true (struct :`R` 1.0 :`A` 1.0) 10.0)
      (`GameplayStatics.SaveGameToSlot` _asplayer_info_save_bp (`self.MySaveSlotName`))
      (return _playerinfo))
    (:`Is Not Valid`
      (`KismetSystemLibrary.PrintString` "error Loading game"))))

(fn `UserConstructionScript`)