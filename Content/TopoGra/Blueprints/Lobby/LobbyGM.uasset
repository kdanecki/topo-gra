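; Lobby game mode that tracks connected lobby players and launches the multiplayer match.
; Joins and logouts update the list of LobbyPC_BP controllers, with new players getting initial setup and a short delay before refresh.
; EveryoneUpdate has each controller refresh its save, gathers their player info, then pushes the full list to every controller's widget.
; StartTheGame shows loading screens on all controllers, then server-travels to Game_L.
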(event `self.K2_PostLogin`
  (params (NewPlayer :type "PlayerController Object Reference"))
  (bind _aslobby_pc_bp (cast `/Game/TopoGra/Blueprints/Lobby/LobbyPC_BP` NewPlayer))
  (`KismetArrayLibrary.Array_Add` (`self.AllPlayerControllers`) _aslobby_pc_bp)
  (`/Game/TopoGra/Blueprints/Lobby/LobbyPC_BP.InitialSetup` _aslobby_pc_bp)
  (`KismetSystemLibrary.Delay` 1.0)
  (`self.EveryoneUpdate`))

(event `self.K2_OnLogout`
  (params (ExitingController :type "Controller Object Reference"))
  (bind _aslobby_pc_bp (cast `/Game/TopoGra/Blueprints/Lobby/LobbyPC_BP` ExitingController))
  (`KismetArrayLibrary.Array_RemoveItem` (`self.AllPlayerControllers`) _aslobby_pc_bp)
  (`self.EveryoneUpdate`))

(event `EveryoneUpdate`
  (`KismetArrayLibrary.Array_Clear` (`self.PlayersInfo`))
  (for _array_element (`self.AllPlayerControllers`)
    (`/Game/TopoGra/Blueprints/Lobby/LobbyPC_BP.RefreshSave` _array_element)
    (`KismetArrayLibrary.Array_Add` (`self.PlayersInfo`) (`/Game/TopoGra/Blueprints/Lobby/LobbyPC_BP.MyPlayerInfo` _array_element)))
  (for _array_element_2 (`self.AllPlayerControllers`)
    (`/Game/TopoGra/Blueprints/Lobby/LobbyPC_BP.UpdateWidget` _array_element_2 (`self.PlayersInfo`))))

(event `StartTheGame`
  (for _array_element (`self.AllPlayerControllers`)
    (`/Game/TopoGra/Blueprints/Lobby/LobbyPC_BP.AddLoadingScreen` _array_element))
  (`KismetSystemLibrary.ExecuteConsoleCommand` "servertravel /Game/TopoGra/Maps/Game_L" (`GameplayStatics.GetPlayerController` 0)))

(fn `UserConstructionScript`)