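; Spawner actor that keeps a single medkit available at its own location and rotation.
; On BeginPlay it spawns one immediately and starts a looping 30-second timer.
; Each tick of the timer respawns the medkit if it no longer exists, or otherwise refills its heal amount to the maximum.
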(event `self.ReceiveBeginPlay`
  (`self.StartSpawning`))

(event `StartSpawning`
  (bind _returnvalue (`KismetSystemLibrary.K2_SetTimerDelegate` (delegate `RefreshMedkit`) 30.0 true))
  (set `self.SpawningTimer` _returnvalue)
  (`self.RefreshMedkit`))

(event `RefreshMedkit`
  (bind _medkit_ref (`self.Medkit_Ref`))
  (`/Engine/EditorBlueprintResources/StandardMacros.IsValid` _medkit_ref
    (:`Is Valid`
      (set `/Game/TopoGra/Blueprints/Medkit/Medkit_BP.HealAmount` (`/Game/TopoGra/Blueprints/Medkit/Medkit_BP.MaxHeal` _medkit_ref) _medkit_ref))
    (:`Is Not Valid`
      (bind _returnvalue (`|SpawnActorFromClass` "/Game/TopoGra/Blueprints/Medkit/Medkit_BP.Medkit_BP_C" (`KismetMathLibrary.MakeTransform` (+ (`self.K2_GetActorLocation`) (0.0 0.0 0.0)) (`self.K2_GetActorRotation`)) "Undefined" "OverrideRootScale" null null))
      (set `self.Medkit_Ref` _returnvalue))))

(fn `UserConstructionScript`)